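; BP_SphereInterpolationMathActor is a sphere actor that animates its material by ping-ponging a blend value.
; The construction script creates a dynamic instance of M_Balls_Inst on the sphere, and BeginPlay picks a random speed multiplier.
; Each TickColor call steps the value by its input times that multiplier, reverses direction at 0 and 1, and writes it to the LerpAlpha parameter.
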(event `self.ReceiveBeginPlay`
  (`parent.ReceiveBeginPlay`)
  (set `self.Multiplier` (`KismetMathLibrary.RandomFloatInRange` 0.1 1.5)))

(event `self.ReceiveTick`
  (params (DeltaSeconds :type "Float (single-precision)"))
  (`parent.ReceiveTick` DeltaSeconds))

(event `Tick Color`
  (params (A :type "Float (double-precision)"))
  (set `self.Value` (+ (`self.Value`) (* (* A (`self.ValueDirection`)) (`self.Multiplier`))))
  (if (<= (`self.Value`) 0.0)
    (set `self.ValueDirection` 1.0))
  (if (>= (`self.Value`) 1.0)
    (set `self.ValueDirection` -1.0))
  (`MaterialInstanceDynamic.SetScalarParameterValue` (`self.Material`) "LerpAlpha" (`self.Value`)))

(fn `UserConstructionScript`
  (`parent.UserConstructionScript`)
  (bind _returnvalue (`PrimitiveComponent.CreateDynamicMaterialInstance` (`self.Sphere`) 0 "/Game/Materials/M_Balls_Inst.M_Balls_Inst" "None"))
  (set `self.Material` _returnvalue))